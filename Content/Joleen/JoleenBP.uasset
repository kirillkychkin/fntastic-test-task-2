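; Joleen character Blueprint that walks to a set destination in one of three movement styles, one per "nest", then plays a temporary Exhaust effect.
; MoveToPoint faces the target and picks the style: gated Tick movement input, timer-driven repeated navmesh moves, or a delay loop.
; The loop alternates moves toward the destination and its opposite point.
; Arrival is a 2D distance check that ignores height.
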(event Custom|EventMoveTypeFirst
  (bind _returnvalue (Transformation|GetActorLocation))
  (bind _destination (Variables|Default|GetDestination))
  ;[1 1 1] Перемещение первого гнезда. Задействует event tick, gate. Вручную задается rotation и добавляется movement input
  (bind _returnvalue_2 (CallFunction|FIndRotation))
  (Utilities|FlowControl|Gate true) ; enters at Open
)

(event Custom|Event%20MoveTypeSecond
  ;[1 1 1] Перемещение второго гнезда. Основано на таймерах. В качестве передвижения используется SImple Move To Location
  (bind _returnvalue (Utilities|Time|SetTimerbyFunctionName 0 "StopTimer" (Variables|Default|GetDuration)))
  (Variables|Default|SetDurationHandle _returnvalue)
  (bind _returnvalue_2 (Utilities|Time|SetTimerbyFunctionName 0 "SimpleMove" (Variables|Default|GetPeriod) true))
  (Variables|Default|SetPeriodHandle _returnvalue_2))

(event Custom|StopTimer
  (bind _returnvalue (Transformation|GetActorLocation))
  (bind _destination (Variables|Default|GetDestination))
  ;[1 1 1] Перемещение второго гнезда. Основано на таймерах. В качестве передвижения используется SImple Move To Location
  (Pawn|Components|CharacterMovement|DisableMovement (Variables|Character|GetCharacterMovement))
  (Utilities|Time|ClearandInvalidateTimerbyHandle (Variables|Default|GetDurationHandle))
  (Utilities|Time|ClearandInvalidateTimerbyHandle (Variables|Default|GetPeriodHandle))
  (if (Math|Vector|Equal(Vector) (Math|Vector|MakeVector (.x _returnvalue) (.y _returnvalue) 0.0) (Math|Vector|MakeVector (.x _destination) (.y _destination) 0.0) 45.0)
    (CallFunction|ArriveatDestination)
    (else
      (bind _returnvalue_2 (Utilities|Time|SetTimerbyFunctionName 0 "StopTimer" (Variables|Default|GetDuration)))
      (Variables|Default|SetDurationHandle _returnvalue_2)
      (bind _returnvalue_3 (Utilities|Time|SetTimerbyFunctionName 0 "SimpleMove" (Variables|Default|GetPeriod) true))
      (Variables|Default|SetPeriodHandle _returnvalue_3))))

(event Custom|EventMoveTypeThird
  (bind _returnvalue (Transformation|GetActorLocation))
  (bind _destination (Variables|Default|GetDestination))
  ;[1 1 1] Перемещение третьего гнезда. Простая конструкиця с Simple Move To Location и задержкой
  (CallFunction|SimpleMove :!label _label)
  (Utilities|FlowControl|Delay 1.0)
  (if (Math|Vector|Equal(Vector) (Math|Vector|MakeVector (.x _returnvalue) (.y _returnvalue) 0.0) (Math|Vector|MakeVector (.x _destination) (.y _destination) 0.0) 45.0)
    (CallFunction|ArriveatDestination)
    (else
      (CallFunction|SimpleMovetoOpposite)
      (Utilities|FlowControl|Delay 0.5)
      (goto _label))))

(event EventTick
  (params (DeltaSeconds :type Float%20%28single-precision%29))
  (bind _returnvalue (Transformation|GetActorLocation))
  (bind _destination (Variables|Default|GetDestination))
  ;[1 1 1] Перемещение первого гнезда. Задействует event tick, gate. Вручную задается rotation и добавляется movement input
  (Utilities|FlowControl|Gate true :!label _label
    (:Exit
      (Pawn|Input|AddMovementInput (Math|Vector|GetForwardVector (stale Custom|EventMoveTypeFirst _returnvalue_2)) 1.0 false)
      (if (Math|Vector|Equal(Vector) (Math|Vector|MakeVector (.x _returnvalue) (.y _returnvalue) 0.0) (Math|Vector|MakeVector (.x _destination) (.y _destination) 0.0) 45.0)
        (CallFunction|ArriveatDestination)
        (goto _label Close)))))

(fn ConstructionScript)

(fn SimpleMove
  (Pawn|Components|CharacterMovement|SetMovementMode (Variables|Character|GetCharacterMovement) "MOVE_NavWalking" 0)
  (AI|Navigation|SimpleMovetoLocation (Pawn|GetController) (Variables|Default|GetDestination)))

(fn SetDestination
  (params (Destination :type Vector))
  (Variables|Default|SetDestination Destination))

(fn MovetoPoint
  (params (MoveType :type Integer))
  (bind _returnvalue (CallFunction|FIndRotation))
  (Transformation|SetActorRotation _returnvalue)
  (switch int MoveType ; Понять какое гнездо и как двигаться
    (:0
      (CallFunction|EventMoveTypeFirst))
    (:1
      (CallFunction|EventMoveTypeSecond))
    (:2
      (CallFunction|SetOppositeDest) ; Противоположная от destination точка относительно места спавна+
      (CallFunction|EventMoveTypeThird))))

(fn CheckDestinationReached
  (bind _output_get (Variables|Default|SetDestination%20Reached (Math|Vector|Equal(Vector) (Variables|Default|GetDestination) (Transformation|GetActorLocation) 5.0)))
  (return _output_get))

(fn SetOppositeDest
  (bind _returnvalue (Transformation|GetActorLocation))
  (bind _returnvalue_2 (Transformation|GetActorLocation))
  (bind _destination (Variables|Default|GetDestination))
  (bind _returnvalue_3 (Math|Vector|GetUnitDirection(Vector) _returnvalue_2 _destination))
  (bind _returnvalue_4 (* _returnvalue_3 -1e+03))
  (bind _returnvalue_5 (+ _returnvalue_4 _returnvalue))
  (Variables|Default|SetOppositeDestination (Math|Vector|MakeVector (.x _returnvalue_5) (.y _returnvalue_5) (.z (Variables|Default|GetDestination)))))

(fn SimpleMovetoOpposite
  (Pawn|Components|CharacterMovement|SetMovementMode (Variables|Character|GetCharacterMovement) "MOVE_NavWalking" 0)
  (AI|Navigation|SimpleMovetoLocation (Pawn|GetController) (Variables|Default|GetOppositeDestination)))

(fn FIndRotation
  (return (Math|Rotator|MakeRotator 0.0 0.0 (.Yaw (Math|Rotator|BreakRotator (Math|Rotator|FindLookatRotation (Transformation|GetActorLocation) (Variables|Default|GetDestination)))))))

(fn ArriveatDestination
  (Components|Activation|Activate (Variables|Default|GetExhaust) false)
  (Utilities|Time|SetTimerbyFunctionName 0 "Deactivate" 5.0))

(fn Deactivate
  (Components|Activation|Deactivate (Variables|Default|GetExhaust)))