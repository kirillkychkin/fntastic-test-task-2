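; NestBP is a stargate-style nest that spawns characters and sends them toward a destination.
; SpawnCharacter plays a particle effect, sound and gate animation with a temporary lit material, then after a delay spawns the configured class in front of its Arrow component, facing along it.
; If the spawned actor is a JoleenBP, it is initialized and, after a short pause, given the destination and told to move with the configured move type.
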(event Custom|Spawn%20Character
  (bind _arrow (Variables|Default|GetArrow))
  (bind _returnvalue (Transformation|GetWorldRotation _arrow))
  (Components|Activation|Activate (Variables|Default|GetParticleSystem) false)
  (Audio|PlaySound2D "/Game/Assets/Sounds/SCIShip_Futuristic_vehicle_crossing_2__ID_0338__BSB.SCIShip_Futuristic_vehicle_crossing_2__ID_0338__BSB" 1.0 1.0 0.0 0 0)
  (Components|Animation|PlayAnimation (Variables|Default|GetSkeletalMesh) "/Game/Nests/Stargate_Anim.Stargate_Anim" false)
  (Rendering|Material|SetMaterial (Variables|Default|GetSkeletalMesh) 0 "/Game/Nests/01_-_Default1Light.01_-_Default1Light")
  (Utilities|FlowControl|Delay 3.0)
  (Rendering|Material|SetMaterial (Variables|Default|GetSkeletalMesh) 0 "/Game/Nests/01_-_Default.01_-_Default")
  (bind _returnvalue_2 (Game|SpawnActorfromClass (Variables|Default|GetClass) (Math|Transform|MakeTransform (+ (Transformation|GetActorLocation) (* (Math|Vector|GetForwardVector _returnvalue) 2.5e+02)) _returnvalue "1,1,1") "AdjustIfPossibleButDontSpawnIfColliding" 0 0))
  (Components|Activation|Deactivate (Variables|Default|GetParticleSystem))
  (bind _asjoleen_bp (Utilities|Casting|CastToJoleenBP _returnvalue_2)) ; Задаем точку назначения и начинаем движение
  (Default|Initial _asjoleen_bp)
  (Utilities|FlowControl|Delay 1.7)
  (Default|SetDestination _asjoleen_bp (Variables|Default|GetCharacterDestination))
  (Default|MovetoPoint _asjoleen_bp (Variables|Default|GetMoveType)))

(fn ConstructionScript)