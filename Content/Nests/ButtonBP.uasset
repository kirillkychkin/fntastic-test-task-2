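; ButtonBP is a clickable button actor that animates a press on its Sphere component.
; On each click it stores the Sphere's current relative location and derives a pressed position 8 units lower in Z.
; The Press timeline then restarts, using its Movement track to lerp the Sphere between the two positions.
; The click triggers nothing beyond this movement.
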(event EventBeginPlay)

(event Collision|EventActorBeginOverlap
  (params (OtherActor :type Actor%20Object%20Reference)))

(event EventTick
  (params (DeltaSeconds :type Float%20%28single-precision%29)))

(event MouseInput|EventActorOnClicked
  (params (ButtonPressed :type Key%20Structure :default "None"))
  (Variables|Default|SetSphereStartLocation (Variables|/Script/Engine.SceneComponent|GetRelativeLocation (Variables|Default|GetSphere)))
  (Variables|Default|SetSpherePressedLocation (Math|Vector|MakeVector (.x (Variables|Default|GetSphereStartLocation)) (.y (Variables|Default|GetSphereStartLocation)) (- (.z (Variables|Default|GetSphereStartLocation)) 8.0)))
  (bind _movement (Timeline|Press PlayFromStart)
    (:Update
      (Transformation|SetRelativeLocation (Variables|Default|GetSphere) (Math|Vector|Lerp(Vector) (Variables|Default|GetSphereStartLocation) (Variables|Default|GetSpherePressedLocation) _movement) false false))))

(fn ConstructionScript)