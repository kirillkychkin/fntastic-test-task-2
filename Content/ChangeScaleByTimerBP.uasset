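; Actor Blueprint that repeatedly grows and shrinks its own scale using timers.
; A looping timer adds a fixed step each period until a duration timer switches to subtraction, and a second duration timer restarts growth.
; Tick caches and prints the current scale; if that cached value equals MaxScale during growth, both active timers are cleared, halting the cycle.
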(event Custom|AddScale
  (Transformation|SetActorScale3D (+ (Transformation|GetActorScale3D) (Variables|Default|GetAdd)))
  (if (Utilities|Operators|EqualEqual (Variables|Default|GetBaseScale) (Variables|Default|GetMaxScale) 0.0)
    (Utilities|Time|ClearandInvalidateTimerbyHandle (Variables|Default|GetDurationHandle))
    (Utilities|Time|ClearandInvalidateTimerbyHandle (Variables|Default|GetPeriodHandle))))

(event Custom|SubtractScale
  (Transformation|SetActorScale3D (- (Transformation|GetActorScale3D) (Variables|Default|GetAdd))))

(event Custom|StopAction2
  (Utilities|Time|ClearandInvalidateTimerbyHandle (Variables|Default|GetDurationHandle2))
  (Utilities|Time|ClearandInvalidateTimerbyHandle (Variables|Default|GetPeriodicHandle2))
  (bind _returnvalue (Utilities|Time|SetTimerbyFunctionName 0 "StopAction" (Variables|Default|GetDuration)))
  (Variables|Default|SetDurationHandle _returnvalue)
  (bind _returnvalue_2 (Utilities|Time|SetTimerbyFunctionName 0 "AddScale" (Variables|Default|GetPeriod) true))
  (Variables|Default|SetPeriodHandle _returnvalue_2))

(event Custom|StopAction
  (Utilities|Time|ClearandInvalidateTimerbyHandle (Variables|Default|GetDurationHandle))
  (Utilities|Time|ClearandInvalidateTimerbyHandle (Variables|Default|GetPeriodHandle))
  (bind _returnvalue (Utilities|Time|SetTimerbyFunctionName 0 "StopAction2" (Variables|Default|GetDuration2)))
  (Variables|Default|SetDurationHandle2 _returnvalue)
  (bind _returnvalue_2 (Utilities|Time|SetTimerbyFunctionName 0 "SubtractScale" (Variables|Default|GetPeriod) true))
  (Variables|Default|SetPeriodicHandle2 _returnvalue_2))

(event EventBeginPlay
  (bind _returnvalue (Utilities|Time|SetTimerbyFunctionName 0 "StopAction" (Variables|Default|GetDuration)))
  (Variables|Default|SetDurationHandle _returnvalue)
  (bind _returnvalue_2 (Utilities|Time|SetTimerbyFunctionName 0 "AddScale" (Variables|Default|GetPeriod) true))
  (Variables|Default|SetPeriodHandle _returnvalue_2))

(event EventTick
  (params (DeltaSeconds :type Float%20%28single-precision%29))
  (bind _output_get (Variables|Default|SetBaseScale (Transformation|GetActorScale3D)))
  (Development|PrintString (Utilities|String|ToString(Vector) _output_get) true true "(R=0.000000,G=0.660000,B=1.000000,A=1.000000)" 0.0))

(fn ConstructionScript)